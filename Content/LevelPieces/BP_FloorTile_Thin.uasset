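; BP_FloorTile_Thin is a floor tile level piece with a thin walkway and a kill zone that ends the game.
; Its construction script gathers four spawn point transforms, then adds a scaled, rotated, offset static mesh at a random one.
; It also stores a separately randomized transform from that set as BP_GameMode's PlayerSpawnPoint.
; A player overlapping KillZone triggers a splash sound and GameComplete.
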(event OnComponentBeginOverlap(KillZone)
  (params (OverlappedComponent :type Primitive%20Component%20Object%20Reference) (OtherActor :type Actor%20Object%20Reference) (OtherComp :type Primitive%20Component%20Object%20Reference) (OtherBodyIndex :type Integer) (bFromSweep :type Boolean) (SweepResult :type Hit%20Result%20Structure%20%28by%20ref%29))
  (bind _asbp_player (Utilities|Casting|CastToBP_Player OtherActor))
  (Audio|PlaySoundatLocation "/Game/Assets/Audio/A_Splash.A_Splash" (Transformation|GetWorldLocation (Variables|/Game/Blueprints/BP_Player.BP_Player_C|GetPlayer _asbp_player)))
  (Default|GameComplete _asbp_player))

(event EventBeginPlay
  (|CallParentFunction))

(event Collision|EventActorBeginOverlap
  (params (OtherActor :type Actor%20Object%20Reference)))

(event EventTick
  (params (DeltaSeconds :type Float%20%28single-precision%29)))

(fn ConstructionScript
  (Utilities|FlowControl|Sequence
    (:then_0
      (CallFunction|GetSpawnLocations)
      (CallFunction|SpawnThinFloor))))

(fn GetSpawnLocations
  (Variables|Default|SetSpawnPoints (Utilities|Array|MakeArray (Transformation|GetRelativeTransform (Variables|Default|GetSpawnPoint5)) (Transformation|GetRelativeTransform (Variables|Default|GetSpawnPoint7)) (Transformation|GetRelativeTransform (Variables|Default|GetSpawnPoint3)) (Transformation|GetRelativeTransform (Variables|Default|GetSpawnPoint9)))))

(fn SpawnThinFloor
  (bind _spawnpoints (Variables|Default|GetSpawnPoints))
  (bind _returnvalue (Utilities|Array|LastIndex _spawnpoints))
  (bind _returnvalue_2 (Math|Random|RandomIntegerinRange 0 _returnvalue))
  (bind _output (Utilities|Array|Get(acopy) _spawnpoints _returnvalue_2))
  (bind _returnvalue_3 (AddComponent|AddStaticMeshComponent false _output))
  (Transformation|SetRelativeScale3D _returnvalue_3 "7.000000,7.000000,7.000000")
  (Transformation|SetWorldRotation _returnvalue_3 "0,-40.000000,0.000000" false false)
  (Transformation|AddWorldOffset _returnvalue_3 "25.000000, 0,230.000000" false false)
  (bind _asbp_game_mode (Utilities|Casting|CastToBP_GameMode (Game|GetGameMode)))
  (Variables|/Game/Blueprints/BP_GameMode.BP_GameMode_C|SetPlayerSpawnPoint _asbp_game_mode _output))